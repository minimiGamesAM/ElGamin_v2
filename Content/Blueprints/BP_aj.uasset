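; BP_aj is a player-controlled pawn or character with movement, mouse look and an interact key.
; Axis inputs drive movement relative to the control rotation's yaw and feed controller yaw and pitch.
; Pressing E calls the Interactuando dispatcher and prints a debug message.
; Possession shows the capsule with its children and enables collision, while unpossession hides them and disables collision, so the body is only present while controlled.
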(event `InputAxis|M_MoverAdelante`
  (params (AxisValue :type "Float (single-precision)"))
  (`self.AddMovementInput` (`KismetMathLibrary.GetForwardVector` (`KismetMathLibrary.MakeRotator` 0.0 0.0 (.yaw (`self.GetControlRotation`)))) AxisValue))

(event `self.ReceiveUnpossessed`
  (params (OldController :type "Controller Object Reference"))
  (bind _capsulecomponent (`self.CapsuleComponent`))
  (`SceneComponent.SetVisibility` _capsulecomponent false true)
  (`PrimitiveComponent.SetCollisionEnabled` _capsulecomponent "NoCollision"))

(event `Key|E`
  (params (Key :type "Key Structure"))
  (:`Pressed`
    (`self.Interactuando`)
    (`KismetSystemLibrary.PrintString` "Llamando Inter")))

(event `self.ReceivePossessed`
  (params (NewController :type "Controller Object Reference"))
  (bind _capsulecomponent (`self.CapsuleComponent`))
  (`SceneComponent.SetVisibility` _capsulecomponent true true)
  (`PrimitiveComponent.SetCollisionEnabled` _capsulecomponent "QueryAndPhysics"))

(event `InputAxis|M_MoverDerecha`
  (params (AxisValue :type "Float (single-precision)"))
  (`self.AddMovementInput` (`KismetMathLibrary.GetRightVector` (`KismetMathLibrary.MakeRotator` 0.0 0.0 (.yaw (`self.GetControlRotation`)))) AxisValue))

(event `InputAxis|M_Girar`
  (params (AxisValue :type "Float (single-precision)"))
  ;[1 1 1] Movimiento con Raton
  (`self.AddControllerYawInput` (stale `InputAxis|M_MirarArriba` AxisValue)))

(event `InputAxis|M_MirarArriba`
  (params (AxisValue :type "Float (single-precision)"))
  ;[1 1 1] Movimiento con Raton
  (`self.AddControllerPitchInput` (stale `InputAxis|M_Girar` AxisValue)))

(fn `UserConstructionScript`)