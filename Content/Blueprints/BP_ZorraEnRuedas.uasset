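; BP_ZorraEnRuedas is a drivable wheeled vehicle pawn that the player can board and leave.
; Axis inputs drive throttle and inverted steering on VehicleMovement and rotate the BrazoCamZorra camera arm.
; Overlapping TriggerSubirseZorra binds BP_aj's Interactuando dispatcher to possess the vehicle, and leaving clears all its bindings.
; Pressing E moves the stored character to LadoDeBajarse and repossesses it.
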(event `InputAxis|M_MoverAdelante`
  (params (AxisValue :type "Float (single-precision)"))
  (`WheeledVehicleMovementComponent.SetThrottleInput` (`self.VehicleMovement`) AxisValue))

(event `InputAxis|M_MoverDerecha`
  (params (AxisValue :type "Float (single-precision)"))
  (`WheeledVehicleMovementComponent.SetSteeringInput` (`self.VehicleMovement`) (* AxisValue -1.0)))

(event `InputAxis|M_MIrarArriba`
  (params (AxisValue :type "Float (single-precision)"))
  (`SceneComponent.K2_AddRelativeRotation` (`self.brazoCamZorra`) (`KismetMathLibrary.MakeRotator` 0.0 0.0 AxisValue) false false))

(event `InputAxis|M_Girar`
  (params (AxisValue :type "Float (single-precision)"))
  (`SceneComponent.K2_AddRelativeRotation` (`self.brazoCamZorra`) (`KismetMathLibrary.MakeRotator` 0.0 AxisValue) false false))

(event `self.triggerSubirseZorra.OnComponentBeginOverlap`
  (params (OverlappedComponent :type "PrimitiveComponent Object Reference") (OtherActor :type "Actor Object Reference") (OtherComp :type "PrimitiveComponent Object Reference") (OtherBodyIndex :type Integer) (bFromSweep :type Boolean) (SweepResult :type "HitResult Structure (by ref)"))
  (bind _asbp_aj (cast `/Game/Blueprints/BP_aj` OtherActor))
  (add `/Game/Blueprints/BP_aj.Interactuando` _asbp_aj (delegate `TomarControlDeZorra`)))

(event `TomarControlDeZorra`
  (set `self.neroAj` (`GameplayStatics.GetPlayerCharacter` 0))
  (`Controller.Possess` (`GameplayStatics.GetPlayerController` 0) self))

(event `Key|E`
  (params (Key :type "Key Structure"))
  (:`Pressed`
    (`self.K2_SetActorTransform` (`self.neroAj`) (`SceneComponent.K2_GetComponentToWorld` (`self.ladoDeBajarse`)) false false)
    (`Controller.Possess` (`GameplayStatics.GetPlayerController` 0) (`self.neroAj`))))

(event `self.triggerSubirseZorra.OnComponentEndOverlap`
  (params (OverlappedComponent :type "PrimitiveComponent Object Reference") (OtherActor :type "Actor Object Reference") (OtherComp :type "PrimitiveComponent Object Reference") (OtherBodyIndex :type Integer))
  (bind _asbp_aj (cast `/Game/Blueprints/BP_aj` OtherActor))
  (clear `/Game/Blueprints/BP_aj.Interactuando` _asbp_aj))

(fn `UserConstructionScript`)